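; Player controller that turns pitch and roll input into rotation of the player pawn.
; Each axis event adds local rotation to player pawn 0, scaled by the axis value, frame delta time and a RotationSpeed variable.
; BeginPlay, Tick and the construction script are empty.
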(event EventBeginPlay)

(event EventTick
  (params (DeltaSeconds :type Float%20%28single-precision%29)))

(event Input|AxisEvents|InputAxisRoll
  (params (AxisValue :type Float%20%28single-precision%29))
  (Transformation|AddActorLocalRotation (Game|Player|GetPlayerPawn 0) (Math|Rotator|MakeRotator (* AxisValue (Utilities|Time|GetWorldDeltaSeconds) (Variables|Default|GetRotationSpeed)) 0.0 0.0) false false))

(event Input|AxisEvents|InputAxisPitch
  (params (AxisValue :type Float%20%28single-precision%29))
  (Transformation|AddActorLocalRotation (Game|Player|GetPlayerPawn 0) (Math|Rotator|MakeRotator 0.0 (* AxisValue (Utilities|Time|GetWorldDeltaSeconds) (Variables|Default|GetRotationSpeed)) 0.0) false false))

(fn ConstructionScript)